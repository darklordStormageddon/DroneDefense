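; BP_Minion1 is a monster minion Character that tracks its proximity to the Nexus and reacts to damage.
; Its construction script stores the nearest TriggerBox as Nexus.
; Overlapping a BP_Nexus sets Close and calls ToggleClose, and ending the overlap clears the flag.
; Incoming damage reduces truncated HP, calls TakeDamage and briefly raises a Hit flag.
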(event `self.OnLanded`
  (params (Hit :type "HitResult Structure (by ref)")))

(event `self.ReceiveBeginPlay`)

(event `self.ReceiveActorBeginOverlap`
  (params (OtherActor :type "Actor Object Reference"))
  (cast `/Game/Collaborators/PS_KSM/Nexus/BP_Nexus` OtherActor)
  (set `self.Close` true)
  (`self.ToggleClose`))

(event `self.ReceiveActorEndOverlap`
  (params (OtherActor :type "Actor Object Reference"))
  (cast `/Game/Collaborators/PS_KSM/Nexus/BP_Nexus` OtherActor)
  (set `self.Close` false))

(event `self.ReceiveAnyDamage`
  (params (Damage :type "Float (single-precision)") (DamageType :type "DamageType Object Reference") (InstigatedBy :type "Controller Object Reference") (DamageCauser :type "Actor Object Reference"))
  (set `self.HP` (`KismetMathLibrary.FTrunc` (- (`self.HP`) Damage)))
  (`self.TakeDamage` Damage)
  (set `self.Hit` true)
  (`KismetSystemLibrary.Delay` 0.1)
  (set `self.Hit` false))

(fn `UserConstructionScript`
  (bind _outactors (`GameplayStatics.GetAllActorsOfClass` "/Script/Engine.TriggerBox"))
  (set `self.Nexus` (`.ReturnValue` (`GameplayStatics.FindNearestActor` (`self.K2_GetActorLocation`) _outactors))))