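; BP_Minion1 is a minion character that tracks the nearest nexus and can be damaged and killed.
; Its construction script caches the nearest TriggerBox as Nexus and the nearest BP_Nexus as RealNexus.
; Overlapping a BP_Nexus sets Close and calls ToggleClose, and ending the overlap clears Close.
; Incoming damage goes through TakeDamage, flags Dead when HP runs out, and briefly pulses the Hit flag.
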(event `self.OnLanded`
  (params (Hit :type "HitResult Structure (by ref)")))

(event `self.ReceiveActorBeginOverlap`
  (params (OtherActor :type "Actor Object Reference"))
  (cast `/Game/Collaborators/PS_KSM/Nexus/BP_Nexus` OtherActor)
  (set `self.Close` true)
  (`self.ToggleClose`))

(event `self.ReceiveTick`
  (params (DeltaSeconds :type "Float (single-precision)")))

(event `self.ReceiveActorEndOverlap`
  (params (OtherActor :type "Actor Object Reference"))
  (cast `/Game/Collaborators/PS_KSM/Nexus/BP_Nexus` OtherActor)
  (set `self.Close` false))

(event `self.ReceiveAnyDamage`
  (params (Damage :type "Float (single-precision)") (DamageType :type "DamageType Object Reference") (InstigatedBy :type "Controller Object Reference") (DamageCauser :type "Actor Object Reference"))
  (`self.TakeDamage` Damage)
  (if (<= (`self.HP`) 0)
    (set `self.Dead` true))
  (set `self.Hit` true)
  (`KismetSystemLibrary.Delay` 0.1)
  (set `self.Hit` false))

(fn `UserConstructionScript`
  (bind _returnvalue (`self.K2_GetActorLocation`))
  (bind _outactors (`GameplayStatics.GetAllActorsOfClass` "/Script/Engine.TriggerBox"))
  (set `self.Nexus` (`.ReturnValue` (`GameplayStatics.FindNearestActor` _returnvalue _outactors)))
  (bind _outactors_2 (`GameplayStatics.GetAllActorsOfClass` "/Game/Collaborators/PS_KSM/Nexus/BP_Nexus.BP_Nexus_C"))
  (bind _asbp_nexus (cast `/Game/Collaborators/PS_KSM/Nexus/BP_Nexus` (`.ReturnValue` (`GameplayStatics.FindNearestActor` _returnvalue _outactors_2))))
  (set `self.RealNexus` _asbp_nexus))