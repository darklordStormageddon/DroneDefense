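; BP_Boss is a boss monster that periodically casts a spell to strengthen the enemies in the level.
; Tick accumulates a timer while no spell is active, then fires the CastSpell dispatcher and spawns a Niagara effect at the Magic component.
; The bound SpellCast event raises Attack, Speed and Defense on every EnemyBase actor, with no revert, so buffs stack.
; A delay then clears the casting flags, restarting the timer.
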(event `self.ReceiveBeginPlay`
  (`parent.ReceiveBeginPlay`)
  (add `self.CastSpell` (delegate `SpellCast`)))

(event `SpellCast`
  (set `self.Casting` true)
  (bind _outactors (`GameplayStatics.GetAllActorsOfClass` "/Script/DroneDefense.EnemyBase"))
  ;[1 1 1] 레벨에 존재하는 적 능력치 증가
  (for _array_element _outactors
    (set `EnemyBase.Attack` (+ (`EnemyBase.Attack` _array_element) 5.0) _array_element)
    (set `EnemyBase.Speed` (+ (`EnemyBase.Speed` _array_element) 50.0) _array_element)
    (set `EnemyBase.Defense` (+ (`EnemyBase.Defense` _array_element) 5.0) _array_element))
  (`KismetSystemLibrary.Delay` 5.0)
  (set `self.Casting` false)
  (set `self.Spell` false))

(event `self.ReceiveTick`
  (params (DeltaSeconds :type "Float (single-precision)"))
  (`parent.ReceiveTick` DeltaSeconds)
  (if (not (`self.Spell`))
    (set `self.SPellTimer` (+ (`self.SPellTimer`) DeltaSeconds))
    (if (>= (`self.SPellTimer`) 10.0)
      (if (not (`self.Casting`))
        (set `self.Spell` true)
        (`self.CastSpell`)
        (`NiagaraFunctionLibrary.SpawnSystemAtLocation` "/Game/Imports/Basic_VFX/Niagara/NS_Basic_1.NS_Basic_1" (`SceneComponent.K2_GetComponentLocation` (`self.Magic`)) (struct) (50.0 50.0 10.0))
        (set `self.SPellTimer` 0.0)))))

(fn `UserConstructionScript`
  (`parent.UserConstructionScript`))