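; BP_Nexus is a damageable Nexus actor that tracks its health and shows it on screen.
; BeginPlay sets MaxHP, then creates a WBP_NexusHP widget, passes it that maximum and adds it to the viewport.
; AnyDamage subtracts damage from HP with no clamp or death handling, and Tick pushes HP to the widget.
; Tick also runs GetAllActorsOfClass for EnemyBase every frame without using the result.
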(event `self.ReceiveBeginPlay`
  (set `self.MaxHP` 4000.0)
  (bind _returnvalue (`|CreateWidget` "/Game/Collaborators/PJ_LHJ/UI/WBP_NexusHP.WBP_NexusHP_C"))
  (bind _output_get (set `self.NexusHP_WDG` _returnvalue))
  (set `/Game/Collaborators/PJ_LHJ/UI/WBP_NexusHP.MaxHP` (`self.MaxHP`) _output_get)
  (`UserWidget.AddToViewport` (`self.NexusHP_WDG`) 0))

(event `self.ReceiveTick`
  (params (DeltaSeconds :type "Float (single-precision)"))
  (set `/Game/Collaborators/PJ_LHJ/UI/WBP_NexusHP.Cur_Nexus_HP` (`self.HP`) (`self.NexusHP_WDG`))
  (`GameplayStatics.GetAllActorsOfClass` "/Script/DroneDefense.EnemyBase"))

(event `self.ReceiveAnyDamage`
  (params (Damage :type "Float (single-precision)") (DamageType :type "DamageType Object Reference") (InstigatedBy :type "Controller Object Reference") (DamageCauser :type "Actor Object Reference"))
  (set `self.HP` (- (`self.HP`) Damage)))

(fn `UserConstructionScript`)