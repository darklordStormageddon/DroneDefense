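; Player controller that manages the wave HUD and pause menu, and supplies the wave range for the game.
; It creates the wave widget hidden on BeginPlay, reveals it on StartPlay and updates it through ChangeWave.
; The Pause input toggles WB_Pause, switching input mode and cursor visibility.
; GetStartWave and GetEndWave read the minimum and maximum levels from the GI_Drone_DF game instance.
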(event `self.ReceiveBeginPlay`
  (bind _returnvalue (`|CreateWidget` "/Game/Collaborators/PJ_LHJ/UI/WBP_WaveUI.WBP_WaveUI_C"))
  (bind _aswbp_wave_ui (cast `/Game/Collaborators/PJ_LHJ/UI/WBP_WaveUI` _returnvalue))
  (bind _output_get (set `self.UI_Wave` _aswbp_wave_ui))
  (`UserWidget.AddToViewport` _output_get 0)
  (`Widget.SetVisibility` _output_get "Hidden"))

(event `InputAction|Pause`
  (params (Key :type "Key Structure"))
  ;[1 1 1] P 입력 시 Pause 위젯 출력_YSH
  (:`Pressed`
    (`/Engine/EditorBlueprintResources/StandardMacros.IsValid` (`self.WidgetRef`)
      (:`Is Valid`
        (if (`Widget.IsInViewport` (`self.WidgetRef`))
          (`Widget.RemoveFromParent` (`self.WidgetRef`))
          (set `self.WidgetRef` null)
          (`WidgetBlueprintLibrary.SetInputMode_GameOnly` self)
          (set `self.bShowMouseCursor` false)
          (`self.SetIgnoreLookInput` false)
          (`self.SetIgnoreMoveInput` false)
          (else
            (`UserWidget.AddToViewport` (`self.WidgetRef`) 0)
            (`WidgetBlueprintLibrary.SetInputMode_GameAndUIEx` self (`self.WidgetRef`) "DoNotLock" false true)
            (set `self.bShowMouseCursor` false))))
      (:`Is Not Valid`
        (bind _returnvalue (`|CreateWidget` "/Game/Collaborators/PS_YSH/WB_Pause.WB_Pause_C" self))
        (bind _output_get (set `self.WidgetRef` _returnvalue))
        (`UserWidget.AddToViewport` _output_get 0)
        (`WidgetBlueprintLibrary.SetInputMode_GameAndUIEx` self null "DoNotLock" true true)
        (set `self.bShowMouseCursor` true)))))

(event `self.ChangeWave`
  (params (NextWave :type Integer))
  (`/Game/Collaborators/PJ_LHJ/UI/WBP_WaveUI.SetWave` (`self.UI_Wave`) NextWave))

(event `self.StartPlay`
  (`parent.StartPlay`)
  (`Widget.SetVisibility` (`self.UI_Wave`) "Visible"))

(fn `GetEndWave`
  (returns (ReturnValue :type Integer))
  (bind _asgi_drone_df (cast `/Game/Collaborators/PS_YSH/GI_Drone_DF` (`GameplayStatics.GetGameInstance`)))
  (return (`/Game/Collaborators/PS_YSH/GI_Drone_DF.Max_Level` _asgi_drone_df)))

(fn `GetStartWave`
  (returns (ReturnValue :type Integer))
  (bind _asgi_drone_df (cast `/Game/Collaborators/PS_YSH/GI_Drone_DF` (`GameplayStatics.GetGameInstance`)))
  (return (`/Game/Collaborators/PS_YSH/GI_Drone_DF.Min_Level` _asgi_drone_df)))

(fn `UserConstructionScript`)