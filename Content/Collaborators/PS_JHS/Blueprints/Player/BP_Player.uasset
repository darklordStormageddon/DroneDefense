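; BP_Player is the player character, with a cooldown-limited gun and drone controls.
; Left click calls Fire, which plays a montage, waits briefly, then spawns a bullet and BP_barrel at the barrel socket.
; The bullet's X/Y direction comes from the offset between two gun sockets.
; BeginPlay generates a drone container, and Enhanced Input actions call drone generation and mode-change functions defined outside these graphs.
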(event `self.ReceiveBeginPlay`
  (`self.GenerateDroneContainer`))

(event `Fire`
  (bind _mesh (`self.Mesh`))
  (bind _returnvalue (`SceneComponent.GetSocketLocation` _mesh "gun_barrelSocket"))
  (bind (_returnvalue_x _returnvalue_y) (`KismetMathLibrary.BreakVector` (- _returnvalue (`SceneComponent.GetSocketLocation` _mesh "gun_barrelSocket_Minus"))))
  (`self.PlayAnimMontage` null)
  (`KismetSystemLibrary.Delay` 0.1)
  (`|SpawnActorFromClass` "/Game/Collaborators/PS_CJH/Bullet/BP_Bullet.BP_Bullet_C" (`KismetMathLibrary.MakeTransform` _returnvalue) "Undefined" "MultiplyWithRoot" null (`KismetMathLibrary.MakeVector` _returnvalue_x _returnvalue_y) null)
  (`|SpawnActorFromClass` "/Game/Collaborators/PS_CJH/Bullet/BP_barrel.BP_barrel_C" (`KismetMathLibrary.MakeTransform` _returnvalue) "Undefined" "MultiplyWithRoot" null null)
  (set `self.LastFireTime` (`GameplayStatics.GetTimeSeconds`)))

(event `EnhancedInput|/Game/Collaborators/PS_JHS/Input/IA_GenerateDrone`
  (params (ActionValue :type Boolean) (ElapsedSeconds :type "Float (double-precision)") (TriggeredSeconds :type "Float (double-precision)") (InputAction :type "InputAction Object Reference" :default "/Game/Collaborators/PS_JHS/Input/IA_GenerateDrone.IA_GenerateDrone"))
  (:`Started`
    (`self.GenerateDroneInput`)))

(event `EnhancedInput|/Game/Collaborators/PS_JHS/Input/IA_ChangeDroneMode`
  (params (ActionValue :type Boolean) (ElapsedSeconds :type "Float (double-precision)") (TriggeredSeconds :type "Float (double-precision)") (InputAction :type "InputAction Object Reference" :default "/Game/Collaborators/PS_JHS/Input/IA_ChangeDroneMode.IA_ChangeDroneMode"))
  (:`Started`
    (`self.ChangeDroneModeInput`)))

(event `Key|LeftMouseButton`
  (params (Key :type "Key Structure"))
  (:`Pressed`
    (if (>= (- (`GameplayStatics.GetTimeSeconds`) (`self.LastFireTime`)) (`self.FireCoolDown`))
      (`self.Fire`)
      (set `self.LastFireTime` (`GameplayStatics.GetTimeSeconds`))))
  (:`Released`
    (`KismetSystemLibrary.K2_ClearAndInvalidateTimerHandle` (`self.Handle`))))

(fn `UserConstructionScript`)