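; BP_Bullet is a projectile that damages enemies on contact.
; Each tick it offsets itself by Vec scaled by BulletSpeed, without sweeping or scaling by delta time.
; When its sphere overlaps an EnemyBase, it applies BulletDamage, spawns BP_Boom at its own transform and destroys itself.
; Other overlaps are ignored, and the bullet otherwise expires after a short delay from BeginPlay.
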(event `self.ReceiveBeginPlay`
  (`KismetSystemLibrary.Delay` 5.0)
  (`self.K2_DestroyActor`))

(event `self.ReceiveTick`
  (params (DeltaSeconds :type "Float (single-precision)"))
  (`self.K2_AddActorWorldOffset` (* (`self.vec`) (`self.BulletSpeed`))))

(event `self.Sphere1.OnComponentBeginOverlap`
  (params (OverlappedComponent :type "PrimitiveComponent Object Reference") (OtherActor :type "Actor Object Reference") (OtherComp :type "PrimitiveComponent Object Reference") (OtherBodyIndex :type Integer) (bFromSweep :type Boolean) (SweepResult :type "HitResult Structure (by ref)"))
  (bind _asenemy_base (cast `EnemyBase` OtherActor))
  (`EnemyBase.TakeDamage` _asenemy_base (`self.BulletDamage`))
  (`|SpawnActorFromClass` "/Game/Collaborators/PS_CJH/Bullet/BP_Boom.BP_Boom_C" (`self.GetTransform` self) "Undefined" "MultiplyWithRoot" null null)
  (`self.K2_DestroyActor`))

(fn `UserConstructionScript`)